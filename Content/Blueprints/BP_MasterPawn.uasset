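; BP_MasterPawn is a pawn Blueprint that gives itself an idle breathing animation and a hit effect.
; On BeginPlay it starts a looping ping-pong scale tween from unit scale to ScaleToVector, eased and ignoring time dilation, and stores it in BreathTweenValue.
; The OnPlayHitAniamtion event spawns the PlayHitPST particle emitter at the pawn's location; no Tick or overlap logic is active.
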(event EventBeginPlay
  (bind _returnvalue (Class|ITween|ActorScalefromtoFull 0.0 "No Name" self "1.000000,1.000000,1.000000" (Math|Conversions|ToVector(Float) (Variables|Default|GetScaleToVector)) true "none" false 0.0 "first" "seconds" (Variables|Default|GetNormalBreathTime) "easeOutCubic" 0 1.0 "pingPong" 0 0 "" 0 "" 0 "" 0 "" false true true false 3.0))
  (Variables|Default|SetBreathTweenValue _returnvalue))

(event EventActorBeginOverlap
  (params (OtherActor :type Actor%20Object%20Reference)))

(event EventTick
  (params (DeltaSeconds :type Float%20%28single-precision%29)))

(event EventOnPlayHitAniamtion
  (Effects|SpawnEmitteratLocation (Variables|Default|GetPlayHitPST) (Transformation|GetActorLocation self) "60.000000, 0, 0"))

(fn ConstructionScript)